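; High-score save data that keeps each player's best score in parallel name and score arrays.
; AddHighScore adds new names or raises an existing score only when beaten, and GetHighScore returns zero for unknown players.
; GetHighScoreList uses an insertion-style pass over five indices, meant to rank the top players, and returns their names and scores.
; ResetScores clears only the score array, leaving names in place.
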(fn ResetScores
  (Utilities|Array|Clear (Variables|Default|GetHighScore)))

(fn AddHighScore
  (params (PlayerName :type String) (HighScore :type Float%20%28single-precision%29))
  (bind _playersnames (Variables|Default|GetPlayersNames))
  (bind _returnvalue (Utilities|Array|FindItem _playersnames PlayerName))
  (if (== _returnvalue -1)
    (Utilities|Array|Add (Variables|Default|GetPlayersNames) PlayerName)
    (Utilities|Array|Add (Variables|Default|GetHighScore) HighScore)
    (elif (< (Utilities|Array|Get(acopy) (Variables|Default|GetHighScore) _returnvalue) HighScore)
      (Utilities|Array|SetArrayElem (Variables|Default|GetHighScore) _returnvalue HighScore)))
  (return))

(fn GetHighScoreList
  (LocalVariables|SetTop5 (Utilities|Array|MakeArray 0 0 0 0 0))
  (for (_array_element _array_index) (Variables|Default|GetHighScore)
    (for (_array_element_2 _array_index_2) (LocalVariables|GetTop5)
      (if (> _array_element (Utilities|Array|Get(acopy) (Variables|Default|GetHighScore) _array_element_2))
        (for _index (range _array_index_2 3)
          (Utilities|Array|SetArrayElem (LocalVariables|GetTop5) (+ _index 1) (Utilities|Array|Get(acopy) (LocalVariables|GetTop5) _index)))
        (Utilities|Array|SetArrayElem (LocalVariables|GetTop5) _array_index_2 _array_index))))
  (for (_array_element_3 _array_index_3) (LocalVariables|GetTop5)
    (Utilities|FlowControl|Sequence
      (:then_0
        (Utilities|Array|SetArrayElem (LocalVariables|GetScores) _array_index_3 (Utilities|Array|Get(acopy) (Variables|Default|GetHighScore) _array_element_3)))
      (:then_1
        (Utilities|Array|SetArrayElem (LocalVariables|GetPlayers) _array_index_3 (Utilities|Array|Get(acopy) (Variables|Default|GetPlayersNames) _array_element_3)))))
  (return (LocalVariables|GetPlayers) (LocalVariables|GetScores)))

(fn GetHighScore
  (params (PlayerName :type String))
  (bind _playersnames (Variables|Default|GetPlayersNames))
  (bind _returnvalue (Utilities|Array|FindItem _playersnames PlayerName))
  (if (== _returnvalue -1)
    (return 0.0)
    (else
      (return (Utilities|Array|Get(acopy) (Variables|Default|GetHighScore) _returnvalue)))))