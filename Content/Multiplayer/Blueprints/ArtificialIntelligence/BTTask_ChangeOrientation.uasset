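; Behavior tree task that turns an AI-controlled fighter to face the first player character along the X axis.
; On execute it caches the controlled C_BaseFigher pawn from its AIC_BaseFighter controller, then picks an orientation by comparing X positions.
; A helper fires the fighter's ChangeOrientationEvent only when the orientation differs, then the task finishes successfully.
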(event EventReceiveExecute
  (params (OwnerActor :type Actor%20Object%20Reference))
  (Utilities|IsValid (Variables|Default|GetControlledFighter)
    (:Is%20Valid
      _)
    (:Is%20Not%20Valid
      (bind _asaic_base_fighter (Utilities|Casting|CastToAIC_BaseFighter OwnerActor))
      (bind _asc_base_figher (Utilities|Casting|CastToC_BaseFigher (Pawn|GetControlledPawn _asaic_base_fighter)))
      (Variables|Default|SetControlledFighter _asc_base_figher)))
  (CallFunction|SetFighterOrientation (Variables|Default|GetControlledFighter) (select (> (.x (Transformation|GetActorLocation (Game|GetPlayerCharacter 0))) (.x (Transformation|GetActorLocation (Variables|Default|GetControlledFighter)))) "NewEnumerator1" "NewEnumerator0"))
  (AI|BehaviorTree|FinishExecute true))

(fn SetFighterOrientation
  (params (Fighter :type C%20Base%20Figher%20Object%20Reference) (DesiredOrientation :type E_FigherOrientation%20Enum))
  (if (Utilities|Enum|NotEqual(Enum) (Variables|/Game/Multiplayer/Blueprints/Characters/C_BaseFigher.C_BaseFigher_C|GetCurrentOrientation Fighter) DesiredOrientation)
    (Default|ChangeOrientationEvent Fighter DesiredOrientation)))