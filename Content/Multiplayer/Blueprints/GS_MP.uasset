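; Multiplayer game state that tracks match and round states, round number and the round countdown.
; A looping timer decrements the time and tells GM_MP when setup ends or playing time runs out.
; RepNotifies on time and state drive tick, music and bell sounds.
; The time RepNotify also randomly spawns bonus BP_Rice pickups on authority, using a random stream seeded each round.
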(event Custom|StartTimer
  (params (RoundTime :type Float%20%28single-precision%29) (TimeStep :type Float%20%28single-precision%29))
  ;[1 1 1] Called by server to start the timer
  (bind _output_get (Variables|Time|SetInitialRoundTime RoundTime))
  (Variables|Time|SetRoundTime _output_get)
  (bind _returnvalue (Utilities|Time|SetTimerbyEvent (delegate Custom|TimerTick) TimeStep true))
  (Variables|Time|SetTimer%20Handle _returnvalue))

(event Custom|ResetTimer
  ;[1 1 1] Reset timer
  (Class|KismetSystemLibrary|ClearTimerHandle (Variables|Time|GetTimer%20Handle)))

(event Custom|TimerTick
  ;[1 1 1] Timer tick
  (switch Utilities|FlowControl|Switch|SwitchonE_MatchState (Variables|Rounds|GetCurrentRoundState)
    (:NewEnumerator2
      (CallFunction|ProcessStartingRoundTime))
    (:NewEnumerator3
      (CallFunction|ProcessPlayingRoundTime))))

(event Custom|UnpauseTimer
  ;[1 1 1] Unpause timer
  (Utilities|Time|UnpauseTimerbyHandle (Variables|Time|GetTimer%20Handle)))

(event Custom|PauseTimer
  ;[1 1 1] Pause timer
  (Utilities|Time|PauseTimerbyHandle (Variables|Time|GetTimer%20Handle)))

(event Custom|Event%20End%20Match
  ;[1 1 1] Matches
  (Variables|Rounds|SetCurrentRoundState "NewEnumerator5"))

(event Custom|Event%20Begin%20Round
  ;[1 1 1] Rounds
  (Variables|Rounds|SetCurrentRoundState "NewEnumerator3")
  (CallFunction|StartTimer 6e+01 1.0))

(event Custom|Event%20Setup%20Round
  ;[1 1 1] Rounds
  (Variables|Rounds|SetCurrentRoundState "NewEnumerator2")
  (Math|Integer|IncrementInt (Variables|Rounds|GetCurrentRoundNumber)
    (:%20%20
      (CallFunction|StartTimer 3.0 1.0)
      (Class|KismetMathLibrary|SeedRandomStream (Variables|Random|GetRandomStream)))))

(event Custom|Event%20End%20Round
  ;[1 1 1] Rounds
  (Variables|Rounds|SetCurrentRoundState "NewEnumerator4"))

(event Custom|Event%20Begin%20Match
  ;[1 1 1] Matches
  (Variables|Rounds|SetCurrentRoundState "NewEnumerator1")
  (Variables|Rounds|SetCurrentRoundNumber 0))

(fn ConstructionScript)

(fn ProcessPlayingRoundTime
  (bind _ended (CallFunction|DecreaseRoundTime))
  (if _ended
    (bind _as_gm_mp (Utilities|GetGameMode)
      (:then
        (Default|EventRoundTimeRunnedOut _as_gm_mp))
      (:Cast%20Failed
        _)))
  (return))

(fn ProcessStartingRoundTime
  (bind _ended (CallFunction|DecreaseRoundTime))
  (if _ended
    (bind _as_gm_mp (Utilities|GetGameMode)
      (:then
        (Default|EventBeginRound _as_gm_mp)))))

(fn DecreaseRoundTime
  (if (<= (- (Variables|Time|GetRoundTime) 1.0) 0.0)
    (CallFunction|PauseTimer)
    (CallFunction|ResetTimer)
    (bind _output_get (Variables|Time|SetRoundTime 0.0))
    (return _output_get true)
    (else
      (bind _output_get_2 (Variables|Time|SetRoundTime (- (Variables|Time|GetRoundTime) 1.0)))
      (return _output_get_2 false))))

(fn OnRepRoundTime
  (switch Utilities|FlowControl|Switch|SwitchonE_MatchState (Variables|Rounds|GetCurrentRoundState)
    (:NewEnumerator2
      (if (> (Variables|Time|GetRoundTime) 0.0)
        (Audio|SpawnSound2D "/Game/Multiplayer/Sound/thomasevd__tick.thomasevd__tick")))
    (:NewEnumerator3
      (Networking|SwitchHasAuthority
        (:Authority
          (if (< (Math|Random|RandomIntegerinRangefromStream 0 99 (Variables|Random|GetRandomStream)) (Variables|Random|GetProbability%20of%20Spawning%20Rice))
            (Game|SpawnActorfromClass "/Game/Multiplayer/Blueprints/Objects/BP_Rice.BP_Rice_C" (Math|Transform|MakeTransform (Math|Vector|MakeVector (Math|Random|RandomFloatinRangefromStream -5.3e+02 5.3e+02 (Variables|Random|GetRandomStream)) 0.0 2.3e+02)) "Undefined" 0 (Math|Random|RandomFloatinRangefromStream 1e+01 5e+01 (Variables|Random|GetRandomStream)) 0)))))))

(fn OnRepCurrentRoundState
  (switch Utilities|FlowControl|Switch|SwitchonE_MatchState (Variables|Rounds|GetCurrentRoundState)
    (:NewEnumerator3
      (bind _returnvalue (Audio|SpawnSound2D "/Game/Multiplayer/Sound/nsstudios__countdown60s.nsstudios__countdown60s"))
      (Variables|Rounds|SetRoundBackgroundMusic _returnvalue))
    (:NewEnumerator4
      (Audio|Components|Audio|Stop (Variables|Rounds|GetRoundBackgroundMusic))
      (Components|DestroyComponent (Variables|Rounds|GetRoundBackgroundMusic))
      (Audio|SpawnSound2D "/Game/Multiplayer/Sound/BoxingBellSound.BoxingBellSound"))))