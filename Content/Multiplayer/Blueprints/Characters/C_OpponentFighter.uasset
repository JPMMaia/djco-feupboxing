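; C_OpponentFighter is the opponent fighter character, a child Blueprint that supplies the green Paper2D flipbook set.
; Its UpdateAnimationFunction event switches on CurrentState and passes the chosen flipbook to ChangeFlipbookFunction.
; The None state picks walk or idle, and Block uses AnimationTimer to move from a start-block flipbook to the held block.
; Other states share one Select, in which taking damage and knockout fall back to idle.
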(event EventUpdateAnimationFunction
  (switch Utilities|FlowControl|Switch|SwitchonE_FigherState (Variables|Default|GetCurrentState)
    (:NewEnumerator0
      ;[1 1 1] Idle / Walk
      (bind _walking (CallFunction|IsWalkingFunction))
      (CallFunction|ChangeFlipbookFunction (select _walking "/Game/Multiplayer/Sprites/Characters/Green/Flipbooks/F_GreenWalk.F_GreenWalk" "/Game/Multiplayer/Sprites/Characters/Green/Flipbooks/F_GreenIdle.F_GreenIdle")))
    (:NewEnumerator1
      ;[1 1 1] Remaining
      (CallFunction|ChangeFlipbookFunction (Utilities|Select :Index (Variables|Default|GetCurrentState) :NewEnumerator0 "/Game/Multiplayer/Sprites/Characters/Green/Flipbooks/F_GreenIdle.F_GreenIdle" :NewEnumerator1 "/Game/Multiplayer/Sprites/Characters/Green/Flipbooks/F_GreenPunch.F_GreenPunch" :NewEnumerator2 "/Game/Multiplayer/Sprites/Characters/Green/Flipbooks/F_GreenKick.F_GreenKick" :NewEnumerator5 "/Game/Multiplayer/Sprites/Characters/Green/Flipbooks/F_GreenBlock.F_GreenBlock" :NewEnumerator4 "/Game/Multiplayer/Sprites/Characters/Green/Flipbooks/F_GreenJump.F_GreenJump" :NewEnumerator6 "/Game/Multiplayer/Sprites/Characters/Green/Flipbooks/F_GreenIdle.F_GreenIdle" :NewEnumerator7 "/Game/Multiplayer/Sprites/Characters/Green/Flipbooks/F_GreenIdle.F_GreenIdle") :!label _label))
    (:NewEnumerator2
      (goto _label))
    (:NewEnumerator5
      ;[1 1 1] Block
      (CallFunction|ChangeFlipbookFunction (select (> (Variables|Default|GetAnimationTimer) 0.1) "/Game/Multiplayer/Sprites/Characters/Green/Flipbooks/F_GreenBlock.F_GreenBlock" "/Game/Multiplayer/Sprites/Characters/Green/Flipbooks/F_GreenStartBlock.F_GreenStartBlock")))
    (:NewEnumerator4
      (goto _label))
    (:NewEnumerator6
      (goto _label))
    (:NewEnumerator7
      (goto _label))))

(fn ConstructionScript
  (|CallParentFunction))