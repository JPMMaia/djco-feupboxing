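; Base projectile actor for multiplayer that damages fighter characters on overlap.
; On the server only, an overlap with anything other than its instigator is cast to C_BaseFigher, which takes a small fixed damage credited to the instigator's PC_MP controller.
; The projectile destroys itself after a hit; overlaps with non-fighter actors only print a debug message.
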(event Collision|EventActorBeginOverlap
  (params (OtherActor :type Actor%20Object%20Reference))
  (Networking|SwitchHasAuthority
    (:Authority
      (if (!= (Variables|Actor|GetInstigator) OtherActor)
        (bind _asc_base_figher (Utilities|Casting|CastToC_BaseFigher OtherActor)
          (:then
            (bind _aspc_mp (Utilities|Casting|CastToPC_MP (Pawn|GetController (Variables|Actor|GetInstigator))))
            (Default|TakeDamage _asc_base_figher 0.1 _aspc_mp)
            (Actor|DestroyActor))
          (:CastFailed
            (Development|PrintString "EventGraph: Failed to cast Actor")))))))

(fn ConstructionScript)