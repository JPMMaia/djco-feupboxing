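; Single-player save game object, going by its SG prefix, that maintains a high score list.
; AddScore appends a score, then loops over the list, printing each entry for debugging and re-sorting within that loop.
; Each sort pass repeatedly extracts the maximum into NewHighScoreList, up to five times, then reinserts those values at the front in descending order without trimming the rest.
; A second print loop is unconnected.
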(fn AddScore
  (params (Score :type Float%20%28single-precision%29))
  (bind _highscorelist (Variables|Default|GetHighScoreList))
  (bind _highscorelist_2 (Variables|Default|GetHighScoreList))
  (bind (_indexofmaxvalue _maxvalue) (Math|Float|MaxOfFloatArray _highscorelist))
  (Utilities|Array|Add _highscorelist_2 Score)
  (for (_array_element _array_index) _highscorelist_2
    (Development|PrintString 0 (Utilities|String|Append "Score " (Utilities|String|ToString(Integer) _array_index) " " (Utilities|String|ToString(Float) _array_element)) true true "(R=0.000000,G=0.660000,B=1.000000,A=1.000000)" 2e+01)
    (Utilities|Array|Clear (LocalVariables|GetNewHighScoreList))
    (for _index (range 0 (Math|Integer|Min(Integer) (Utilities|Array|LastIndex (Variables|Default|GetHighScoreList)) 4))
      (Utilities|Array|Add (LocalVariables|GetNewHighScoreList) _maxvalue)
      (Utilities|Array|RemoveIndex (Variables|Default|GetHighScoreList) _indexofmaxvalue))
    (for (_array_element_2 _array_index_2) (LocalVariables|GetNewHighScoreList)
      (Utilities|Array|Insert (Variables|Default|GetHighScoreList) _array_element_2 _array_index_2))))