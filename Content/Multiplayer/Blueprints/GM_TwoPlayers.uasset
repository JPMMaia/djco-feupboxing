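; Two-player multiplayer game mode, going by its name, that handles a round win and ends the match.
; RoundWon relays to MulticastRoundWon, though the call shows Score fixed at zero and no PlayerController passed.
; The multicast event plays a boxing bell, prints the winner's ID and updates the high score in GI_MP.
; After a short delay it opens L_MainMenu, or prints an error if the game instance cast fails.
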(event Custom|MulticastRoundWon
  (params (Player%20Controller :type Player%20Controller%20Object%20Reference) (Score :type Float%20%28single-precision%29))
  (bind _playerstate (Variables|/Script/Engine.Controller|GetPlayerState Player%20Controller))
  ;[1 1 1] Called by the server to notify everyone that a player has won a round
  (Audio|SpawnSound2D "/Game/Multiplayer/Sound/BoxingBellSound.BoxingBellSound")
  (Development|PrintString (Utilities|String|Append "Game won by" (Utilities|String|ToString(Integer) (Variables|/Script/Engine.PlayerState|GetPlayerId _playerstate))) true true "(R=0.000000,G=0.660000,B=1.000000,A=1.000000)" 2e+01)
  (bind _asgi_mp (Utilities|Casting|CastToGI_MP (Game|GetGameInstance))
    (:then
      (Default|UpdateHighScore _asgi_mp (Variables|/Script/Engine.PlayerState|GetPlayerName _playerstate) Score)
      (Utilities|FlowControl|Delay 2.0)
      (Game|OpenLevel(byName) "L_MainMenu"))
    (:CastFailed
      (Development|PrintString "EventGraph: Failed to cast Game Instance"))))

(event Custom|RoundWon
  (params (PlayerController :type Player%20Controller%20Object%20Reference) (Score :type Float%20%28single-precision%29))
  ;[1 1 1] Called by the server to notify everyone that a player has won a round
  (CallFunction|MulticastRoundWon 0 0.0))

(fn ConstructionScript
  (|CallParentFunction))