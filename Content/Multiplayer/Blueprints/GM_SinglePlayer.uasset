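; Single-player game mode for a one-on-one fight between the player and an AI-controlled fighter.
; Begins the match on play and resets both fighters to their start actors with opposite orientations, finding the AI's pawn through its controller.
; Match end notifies the game state and each player state of the result, saves the high score through the game instance, then opens the main menu after a short delay.
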(event EventBeginPlay
  ;[1 1 1] Begin Play
  (CallFunction|EventBeginMatch))

(event EventEventEndMatch
  (params (Winner :type PS%20MP%20Object%20Reference))
  ;[1 1 1] End Match
  (bind _asgs_mp (Utilities|Casting|CastToGS_MP (Game|GetGameState)))
  (Default|EventEndMatch _asgs_mp)
  (for _array_element (Variables|/Script/Engine.GameState|GetPlayerArray _asgs_mp)
    (bind _asps_mp (Utilities|Casting|CastToPS_MP _array_element))
    (Default|EventEndMatch _asps_mp (== _asps_mp Winner))
    (CallFunction|SaveHighScore)
    (Utilities|FlowControl|Delay 2.0)
    (Game|OpenLevel(byName) "L_MainMenu")))

(event EventResetPlayers
  ;[1 1 1] Reset Players
  (bind _playercharacter (CallFunction|GetPlayerCharacter))
  (Default|Reset _playercharacter (Transformation|GetActorLocation (Utilities|Array|Get(acopy) (Variables|Default|GetPlayer1))) "NewEnumerator1")
  (bind _controlledcharacter (CallFunction|GetAICharacter))
  (Default|Reset _controlledcharacter (Transformation|GetActorLocation (Utilities|Array|Get(acopy) (Variables|Default|GetPlayer2))) "NewEnumerator0"))

(fn ConstructionScript
  (|CallParentFunction))

(fn GetPlayerCharacter
  (bind _asc_base_figher (Utilities|Casting|CastToC_BaseFigher (Game|GetPlayerCharacter 0))
    (:then
      _)
    (:CastFailed
      (Development|PrintString "Failed to cast character")))
  (return _asc_base_figher))

(fn GetAICharacter
  (bind _outactors (Actor|GetAllActorsOfClass "/Game/Multiplayer/Blueprints/ArtificialIntelligence/AIC_BaseFighter.AIC_BaseFighter_C"))
  (bind _asc_base_figher (Utilities|Casting|CastToC_BaseFigher (Pawn|GetControlledPawn (Utilities|Array|Get(acopy) _outactors)))
    (:then
      _)
    (:CastFailed
      (Development|PrintString "Failed to cast pawn")))
  (return _asc_base_figher))

(fn SaveHighScore
  (bind _asgi_mp (Utilities|Casting|CastToGI_MP (Game|GetGameInstance))
    (:then
      (Default|SaveSinglePlayerHighScore _asgi_mp))
    (:CastFailed
      (Development|PrintString "Failed to cast Game Instance"))))