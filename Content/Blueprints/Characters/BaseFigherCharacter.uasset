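; Base 2D fighter character that walks along X, jumps, punches, kicks and blocks, with flipbook animation.
; An action state locks out movement and other actions; each tick picks the flipbook, faces the velocity direction and clears timed attacks or finished jumps.
; A hand-socket collider is enabled on punch; overlaps during Punch damage other fighters, reduced by blocking.
; Kick deals no damage, and UpdateCollision, which would disable the collider, is never called.
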(event Collision|EventActorBeginOverlap
  (params (OtherActor :type Actor%20Object%20Reference))
  (bind _asbase_figher_character (Utilities|Casting|CastToBaseFigherCharacter OtherActor)
    (:then
      (Utilities|IsPunching
        (:True
          (Actions|TakeDamage _asbase_figher_character 0.5))))
    (:CastFailed
      (Development|PrintString "Failed to cast to Base Fighter Character"))))

(event EventTick
  (params (DeltaSeconds :type Float%20%28single-precision%29))
  (Utilities|UpdateCharacter DeltaSeconds))

(event EventOnJumped
  (Utilities|ChangeStateifNotBusy "NewEnumerator4"))

(fn ConstructionScript
  (Class|SceneComponent|Attachto (Variables|Default|GetPunchCollision) (Variables|Default|GetSprite) "HandSocket" "KeepRelativeOffset" true))

(fn MoveRight
  (params (AxisValue :type Float%20%28single-precision%29))
  (Utilities|IsBusy
    (:False
      (Pawn|Input|AddMovementInput "1.000000, 0, 0" (Math|Float|Clamp(Float) AxisValue -1.0) false))))

(fn Punch
  (Utilities|ChangeStateifNotBusy "NewEnumerator1"
    (:NewState
      (Collision|SetCollisionEnabled (Variables|Default|GetPunchCollision) "QueryAndPhysics"))))

(fn Kick
  (Utilities|ChangeStateifNotBusy "NewEnumerator2"))

(fn StartBlocking
  (Utilities|ChangeStateifNotBusy "NewEnumerator5"))

(fn EndBlocking
  (if (Utilities|Enum|Equal(Enum) (Variables|Figher|GetCurrentState) "NewEnumerator5")
    (Utilities|FlowControl|Sequence
      (:then_0
        (Variables|Figher|SetCurrentState "NewEnumerator0"))
      (:then_1
        (Utilities|ResetAnimationTimer)))))

(fn TakeDamage
  (params (Value :type Float%20%28single-precision%29))
  (Variables|Figher|SetHealth (- (Variables|Figher|GetHealth) (Math|Float|SelectFloat (* Value (- 1.0 (Variables|Figher|GetBlockingPower))) Value (Utilities|Enum|Equal(Enum) (Variables|Figher|GetCurrentState) "NewEnumerator5")))))