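; TestCharacter is a 2D flipbook character Blueprint that moves along the world X axis from the MoveRight input.
; The same input turns the Sprite to face the travel direction by setting its world rotation, keeping the last facing at zero input.
; Tick calls UpdateAnimation, which checks velocity through IsMoving but is unfinished: the branch is empty and the SetFlipbook node is unconnected, with DraftIdle as both options.
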(event EventBeginPlay)

(event EventActorBeginOverlap
  (params (OtherActor :type Actor%20Object%20Reference)))

(event EventTick
  (params (DeltaSeconds :type Float%20%28single-precision%29))
  (CallFunction|UpdateAnimation))

(event Input|AxisEvents|InputAxisMoveRight
  (params (AxisValue :type Float%20%28single-precision%29))
  (Pawn|Input|AddMovementInput "1.000000, 0, 0" AxisValue false)
  (CallFunction|UpdateRotation AxisValue))

(fn ConstructionScript)

(fn UpdateAnimation
  (bind _ismoving (CallFunction|IsMoving))
  (if _ismoving
    _))

(fn UpdateRotation
  (params (InputAxis%20MoveRight :type Float%20%28single-precision%29))
  (if (!= InputAxis%20MoveRight 0.0)
    (Transformation|SetWorldRotation (Variables|Default|GetSprite) (select (> InputAxis%20MoveRight 0.0) "0,0.000000,0" "0,180.000000,0") false false))
  (return))

(fn IsMoving
  (return (> (Math|Vector|VectorLength (Transformation|GetVelocity)) 0.0)))